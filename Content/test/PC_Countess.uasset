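; PC_Countess is a player controller that lets the player submit story text when the Countess character reports Grux in range.
; It binds to the pawn's range event, shows a WBP_Player_Story widget on entry, then after a short delay switches to UI-only input with a cursor.
; Committed text goes to the character, clears the field and restores game input.
; Leaving range removes the widget and restores game input.
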(event Custom|ManagePlayerStoryWdget
  (params (bInRange :type Boolean))
  (if bInRange
    (bind _returnvalue (UserInterface|CreateWidget "/Game/test/UI/WBP_Player_Story.WBP_Player_Story_C"))
    (bind _output_get (Variables|Default|SetWBPPlayerStory _returnvalue))
    (UserInterface|Viewport|AddtoViewport _output_get 0)
    (EventDispatchers|AssignPlayerCommittedStory (Variables|Default|GetWBPPlayerStory) (delegate Custom|OnPlayerCommittedStory))
    (Utilities|FlowControl|Delay 2.0)
    (Input|SetInputModeUIOnly self (Variables|Default|GetWBPPlayerStory) "DoNotLock")
    (Variables|Default|SetbShowMouseCursor true)
    (else
      (Utilities|IsValid (Variables|Default|GetWBPPlayerStory)
        (:Is%20Valid
          (Widget|RemovefromParent (Variables|Default|GetWBPPlayerStory))
          (Input|SetInputModeGameOnly self)
          (Variables|Default|SetbShowMouseCursor false))))))

(event Custom|OnPlayerCommittedStory
  (params (PlayerText :type Text))
  (Default|EventPlayerCommittedStory (Variables|Default|GetPlayerCharacter) PlayerText)
  (Input|SetInputModeGameOnly self)
  (Rendering|Components|TextRender|SetText (Variables|/Game/test/UI/WBP_Player_Story.WBP_Player_Story_C|GetPlayerInput (Variables|Default|GetWBPPlayerStory)) ""))

(event EventBeginPlay
  (bind _output_get (Variables|Default|SetPlayerCharacter (.AsCountess%20Player%20Character (Utilities|Casting|CastToCountessPlayerCharacter (Pawn|GetControlledPawn)))))
  (EventDispatchers|BindEventtoGruxinRange _output_get (delegate Custom|ManagePlayerStoryWdget)))

(fn ConstructionScript)